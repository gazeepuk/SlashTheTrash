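; Base Gameplay Ability for ultimate skills that commits, then plays an attack montage on the avatar's skeletal mesh.
; Gameplay event listeners for start, perform and end attack apply the attacking-state effect, call PerformAbilityAction and remove the effect via its stored handle.
; The ability ends on failed commit, missing mesh or any montage completion, blend-out, interruption or notify callback, with effect removal repeated on end as cleanup.
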(event Ability|EventActivateAbility
  (bind _returnvalue (Ability|GetAbilitySystemComponentfromActorInfo))
  (bind _returnvalue_2 (Ability|GetAvatarActorfromActorInfo))
  (bind _returnvalue_3 (Ability|GetAbilitySystemComponentfromActorInfo))
  (bind _returnvalue_4 (Actor|GetComponentbyClass _returnvalue_2 "/Script/Engine.SkeletalMeshComponent"))
  (bind _returnvalue_5 (Ability|CommitAbility))
  (if _returnvalue_5
    (Utilities|IsValid _returnvalue_4
      (:Is%20Valid
        (Animation|Montage|PlayMontage _returnvalue_4 (Variables|Default|GetAbilityMontage)
          (:then
            (Ability|Tasks|WaitGameplayEvent "(TagName=\"Event.Combat.StartAttack\")" 0
              (:then
                (Ability|Tasks|WaitGameplayEvent "(TagName=\"Event.Combat.PerformAttack\")" 0
                  (:then
                    (Ability|Tasks|WaitGameplayEvent "(TagName=\"Event.Combat.EndAttack\")" 0
                      (:EventReceived
                        (Utilities|IsValid _returnvalue_3
                          (:Is%20Valid
                            (GameplayEffects|RemoveActiveGameplayEffect _returnvalue_3 (Variables|Default|GetActiveEffectHandle) -1))))))
                  (:EventReceived
                    (Class|STTAttackAbilityBase|PerformAbilityAction))))
              (:EventReceived
                (Utilities|IsValid _returnvalue
                  (:Is%20Valid
                    (bind _returnvalue_6 (GameplayEffects|ApplyGameplayEffectToSelf :self _returnvalue :GameplayEffectClass "/Game/Blueprints/AbilitySystem/Effects/States/GE_AttackingState.GE_AttackingState_C" :Level 1.0))
                    (Variables|Default|SetActiveEffectHandle _returnvalue_6))))))
          (:OnCompleted
            (Ability|EndAbility :!label _label))
          (:OnBlendOut
            (goto _label))
          (:OnInterrupted
            (goto _label))
          (:OnNotifyBegin
            (goto _label))
          (:OnNotifyEnd
            (goto _label))))
      (:Is%20Not%20Valid
        (goto _label)))
    (else
      (goto _label))))

(event Ability|EventOnEndAbility
  (params (bWasCancelled :type Boolean))
  (bind _returnvalue (Ability|GetAbilitySystemComponentfromActorInfo))
  (Utilities|IsValid _returnvalue
    (:Is%20Valid
      (GameplayEffects|RemoveActiveGameplayEffect _returnvalue (Variables|Default|GetActiveEffectHandle) -1))))