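; GA_Dismay is an ultimate attack gameplay ability that supplies an area search for damageable actors around its avatar.
; TraceDamageableActors runs a zero-length multi-sphere trace of AbilityRadius on the Camera channel, ignoring the avatar and drawing debug shapes.
; Blocking hits implementing DamageableInterface are added uniquely to CollapsedActors, which is returned.
; The event graph holds only disabled activate and end events, so no effect is applied here.
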(event Ability|EventActivateAbility
  (|CallParentFunction) ; This node is disabled and will not be called.\nDrag off pins to build functionality.
)

(event Ability|EventOnEndAbility
  (params (bWasCancelled :type Boolean))
  (|CallParentFunction bWasCancelled) ; This node is disabled and will not be called.\nDrag off pins to build functionality.
)

(fn TraceDamageableActors
  (bind _returnvalue (Ability|GetAvatarActorfromActorInfo))
  (bind _returnvalue_2 (Transformation|GetActorLocation _returnvalue))
  (bind _outhits (Collision|MultiSphereTraceByChannel _returnvalue_2 _returnvalue_2 (LocalVariables|GetAbilityRadius) "TraceTypeQuery2" false (Utilities|Array|MakeArray _returnvalue) "ForDuration"))
  (for _array_element _outhits
    (if (.bBlockingHit (Collision|BreakHitResult _array_element))
      (Utilities|IsValid (.HitActor (Collision|BreakHitResult _array_element))
        (:Is%20Valid
          (if (Utilities|DoesObjectImplementInterface (.HitActor (Collision|BreakHitResult _array_element)) "/Script/SlashTheTrash.DamageableInterface")
            (Utilities|Array|AddUnique (LocalVariables|GetCollapsedActors) (.HitActor (Collision|BreakHitResult _array_element))))))))
  (return (LocalVariables|GetCollapsedActors)))