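; GA_ComboBase is a base gameplay ability for combo attacks that plays a montage and applies an attacking-state effect.
; Gameplay events trigger PerformAbilityAction and remove the effect at attack end.
; Montage completion also removes it, ends the ability and resets the player's last combo class.
; A helper sphere-traces ahead of the avatar and returns unique actors implementing DamageableInterface, with debug drawing enabled.
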(event Ability|EventActivateAbility
  (bind _returnvalue (Ability|GetAbilitySystemComponentfromActorInfo))
  (bind _returnvalue_2 (Ability|GetAbilitySystemComponentfromActorInfo))
  (|PlayMontageandWaitProxy "None" (Variables|Default|GetAbilityMontage) 1.0 "None" true 1.0 0.0 false
    (:then
      (Utilities|IsValid _returnvalue
        (:Is%20Valid
          (bind _returnvalue_3 (GameplayEffects|ApplyGameplayEffectToSelf :self _returnvalue :GameplayEffectClass "/Game/Blueprints/AbilitySystem/Effects/States/GE_AttackingState.GE_AttackingState_C" :Level 1.0))
          (Variables|Default|SetActiveEffectHandle _returnvalue_3)
          (Ability|Tasks|WaitGameplayEvent "(TagName=\"Event.Combat.PerformAttack\")" 0
            (:then
              (Ability|Tasks|WaitGameplayEvent "(TagName=\"Event.Combat.EndAttack\")" 0
                (:EventReceived
                  (Utilities|IsValid _returnvalue_2 :!label _label
                    (:Is%20Valid
                      (GameplayEffects|RemoveActiveGameplayEffect _returnvalue_2 (Variables|Default|GetActiveEffectHandle) -1))))))
            (:EventReceived
              (Class|STTAttackAbilityBase|PerformAbilityAction))))))
    (:OnCompleted
      (Ability|EndAbility)
      (CallFunction|ResetLastComboClass)
      (goto _label))))

(event Ability|EventOnEndAbility
  (params (bWasCancelled :type Boolean)))

(fn TraceDamageableActors
  (bind _returnvalue (Ability|GetAvatarActorfromActorInfo))
  (bind _returnvalue_2 (Transformation|GetActorLocation _returnvalue))
  (Utilities|IsValid _returnvalue
    (:Is%20Valid
      (bind _outhits (Collision|MultiSphereTraceByChannel _returnvalue_2 (+ _returnvalue_2 (* (Transformation|GetActorForwardVector _returnvalue) 8e+01)) 75.0 "TraceTypeQuery2" false (Utilities|Array|MakeArray (Ability|GetAvatarActorfromActorInfo)) "ForDuration" true "(R=1.000000,G=0.000000,B=0.000000,A=1.000000)" "(R=0.000000,G=1.000000,B=0.000000,A=1.000000)" 0.5))
      (for _array_element _outhits
        (if (.bBlockingHit (Collision|BreakHitResult _array_element))
          (Utilities|IsValid (.HitActor (Collision|BreakHitResult _array_element))
            (:Is%20Valid
              (if (Utilities|DoesObjectImplementInterface (.HitActor (Collision|BreakHitResult _array_element)) "/Script/SlashTheTrash.DamageableInterface")
                (Utilities|Array|AddUnique (LocalVariables|GetCollapsedActors) (.HitActor (Collision|BreakHitResult _array_element))))))))
      (return (LocalVariables|GetCollapsedActors)))))

(fn ResetLastComboClass
  (bind _returnvalue (Class|STTGameplayAbilityBase|GetSTTPlayerCharacterfromActorInfo))
  (Utilities|IsValid _returnvalue
    (:Is%20Valid
      (Class|STTPlayerCharacter|ResetLastComboAttackClass _returnvalue))))