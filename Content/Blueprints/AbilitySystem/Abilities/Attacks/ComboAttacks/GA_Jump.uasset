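; GA_Jump is a Gameplay Ability that makes the avatar Character jump.
; Activation is allowed only when the avatar is a valid Character and its CanJump passes.
; On activation it commits the ability, calls Jump, then applies GE_JumpState to the character's own Ability System Component.
; The graph never calls EndAbility, and its OnEndAbility handler is empty.
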(event Ability|EventActivateAbility
  (bind _returnvalue (Ability|CommitAbility))
  (if _returnvalue
    (bind _ascharacter (Utilities|Casting|CastToCharacter (Ability|GetAvatarActorfromActorInfo)))
    (Character|Jump _ascharacter)
    (Utilities|IsValid (Ability|GetAbilitySystemComponent _ascharacter)
      (:Is%20Valid
        (GameplayEffects|ApplyGameplayEffectToSelf :self (Ability|GetAbilitySystemComponent _ascharacter) :GameplayEffectClass "/Game/Blueprints/AbilitySystem/Effects/GE_JumpState.GE_JumpState_C" :Level 1.0)))))

(event Ability|EventOnEndAbility
  (params (bWasCancelled :type Boolean)))

(fn K2CanActivateAbility
  (params (ActorInfo :type Gameplay%20Ability%20Actor%20Info%20Structure) (Handle :type Gameplay%20Ability%20Spec%20Handle%20Structure))
  (bind _avataractor (Utilities|Struct|BreakGameplayAbilityActorInfo ActorInfo))
  (Utilities|IsValid _avataractor
    (:Is%20Valid
      (bind _ascharacter (Utilities|Casting|CastToCharacter _avataractor)
        (:then
          (return "" (Character|CanJump _ascharacter)))
        (:CastFailed
          _)))
    (:Is%20Not%20Valid
      _))
  (return "" false))