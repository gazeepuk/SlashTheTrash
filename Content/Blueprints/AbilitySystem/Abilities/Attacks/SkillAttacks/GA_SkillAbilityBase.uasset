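; Base gameplay ability for skill attacks that plays AbilityMontage and drives the attack through gameplay events.
; StartAttack applies GE_AttackingState to self and stores its handle, PerformAttack calls PerformAbilityAction, and EndAttack removes the effect.
; The ability ends when the montage completes, blends out, is interrupted or is cancelled.
; OnEndAbility is empty, so only the EndAttack event removes the attacking effect here.
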(event Ability|EventActivateAbility
  (bind _returnvalue (Ability|GetAbilitySystemComponentfromActorInfo))
  (bind _returnvalue_2 (Ability|GetAbilitySystemComponentfromActorInfo))
  (|PlayMontageandWaitProxy "None" (Variables|Default|GetAbilityMontage) 1.0 "None" true 1.0 0.0 false
    (:then
      (Ability|Tasks|WaitGameplayEvent "(TagName=\"Event.Combat.StartAttack\")" 0
        (:then
          (Ability|Tasks|WaitGameplayEvent "(TagName=\"Event.Combat.PerformAttack\")" 0
            (:then
              (Ability|Tasks|WaitGameplayEvent "(TagName=\"Event.Combat.EndAttack\")" 0
                (:EventReceived
                  (Utilities|IsValid _returnvalue_2
                    (:Is%20Valid
                      (GameplayEffects|RemoveActiveGameplayEffect _returnvalue_2 (Variables|Default|GetActiveEffectHandle) -1))))))
            (:EventReceived
              (Class|STTAttackAbilityBase|PerformAbilityAction))))
        (:EventReceived
          (Utilities|IsValid _returnvalue
            (:Is%20Valid
              (bind _returnvalue_3 (GameplayEffects|ApplyGameplayEffectToSelf :self _returnvalue :GameplayEffectClass "/Game/Blueprints/AbilitySystem/Effects/States/GE_AttackingState.GE_AttackingState_C" :Level 1.0))
              (Variables|Default|SetActiveEffectHandle _returnvalue_3))))))
    (:OnCompleted
      (Ability|EndAbility :!label _label))
    (:OnBlendOut
      (goto _label))
    (:OnInterrupted
      (goto _label))
    (:OnCancelled
      (goto _label))))

(event Ability|EventOnEndAbility
  (params (bWasCancelled :type Boolean)))